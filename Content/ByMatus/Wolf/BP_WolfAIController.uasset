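; BP_WolfAIController is the AI controller for the wolf, driven by the BT_Wolf behavior tree.
; On BeginPlay it runs the tree and stores the controlled pawn's location in the StartLocationKey blackboard key.
; Each AI Perception target update writes the reported actor to TargetActor, without checking whether it was sensed or lost.
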(event OnTargetPerceptionUpdated(AIPerception)
  (params (Actor :type Actor%20Object%20Reference) (Stimulus :type AI%20Stimulus%20Structure))
  (AI|Components|Blackboard|SetValueasObject (Variables|Default|GetBlackboard) (Variables|Default|GetTargetActor) Actor))

(event EventBeginPlay
  (AI|RunBehaviorTree "/Game/ByMatus/Wolf/BT_Wolf.BT_Wolf")
  (AI|Components|Blackboard|SetValueasVector (Variables|Default|GetBlackboard) (Variables|Default|GetStartLocationKey) (Transformation|GetActorLocation (Pawn|GetControlledPawn self))))

(fn ConstructionScript)