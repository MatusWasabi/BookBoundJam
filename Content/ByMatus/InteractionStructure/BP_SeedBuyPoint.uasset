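; BP_SeedBuyPoint is a shop trigger that sells a seed when something overlaps its Box.
; The overlap asynchronously loads the soft Seed class, then spawns it at the point's own transform.
; It then deducts a hardcoded price through MoneySubSytem and tells PlayerHUD to update.
; The graph checks neither the overlapping actor nor the available balance.
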(event OnComponentBeginOverlap(Box)
  (params (OverlappedComponent :type Primitive%20Component%20Object%20Reference) (OtherActor :type Actor%20Object%20Reference) (OtherComp :type Primitive%20Component%20Object%20Reference) (OtherBodyIndex :type Integer) (bFromSweep :type Boolean) (SweepResult :type Hit%20Result%20Structure%20%28by%20ref%29))
  (bind _class (Utilities|AsyncLoadClassAsset (Variables|Default|GetSeed))
    (:Completed
      (bind _asactor (Utilities|Casting|CastToActorClass _class))
      (Game|SpawnActorfromClass _asactor (Transformation|GetActorTransform self) "Undefined" 0 0)
      (Class|MoneySubSytem|Decrease (Subsystems|GetMoneySubSytem) 100)
      (bind _asplayer_hud (Utilities|Casting|CastToPlayerHUD (HUD|GetHUD (Game|GetPlayerController 0))))
      (Default|CallUpdateHUD _asplayer_hud))))

(event EventBeginPlay)

(event Collision|EventActorBeginOverlap
  (params (OtherActor :type Actor%20Object%20Reference)))

(event EventTick
  (params (DeltaSeconds :type Float%20%28single-precision%29)))

(fn ConstructionScript)